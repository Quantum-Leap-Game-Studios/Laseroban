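; Blueprint function library of shared helpers, covering more than the conversions its name suggests.
; Direction helpers convert EDirection to and from unit vectors, test for the X axis and cycle clockwise.
; UI helpers detect viewport mouse movement, focus widgets, and switch player input, input mode and cursor for pausing without pausing the game itself.
; Utilities add type-tagged colored debug printing, three-color interpolation over an interval and a checked GI_Global cast.
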(fn `EDirectionNext`
  (params (Direction :type "/Game/Blueprints/Enums/E_Direction Enum" :default "NewEnumerator0"))
  (returns (NewDirection :type "/Game/Blueprints/Enums/E_Direction Enum"))
  (bind _array (`|MakeArray` "NewEnumerator0" "NewEnumerator3" "NewEnumerator1" "NewEnumerator2" :!type "/Game/Blueprints/Enums/E_Direction Enum"))
  (bind _returnvalue (`KismetArrayLibrary.Array_Find` _array Direction))
  (return (select `bool` (== _returnvalue 3) :`false` (`|GetArrayItem` _array (+ _returnvalue 1)) :`true` "NewEnumerator0")))

(fn `EDirectionOnXAxis`
  (params (Direction :type "/Game/Blueprints/Enums/E_Direction Enum" :default "NewEnumerator0"))
  (returns (`Return Value` :type Boolean))
  (return (or (`|EnumEquality` Direction "NewEnumerator0") (`|EnumEquality` Direction "NewEnumerator1"))))

(fn `EDirectionToVector`
  (params (Direction :type "/Game/Blueprints/Enums/E_Direction Enum" :default "NewEnumerator0"))
  (returns (Vector :type "Vector Structure"))
  (return (select `/Game/Blueprints/Enums/E_Direction` Direction :`NewEnumerator0` (1.0 0.0 0.0) :`NewEnumerator1` (-1.0 0.0 0.0) :`NewEnumerator2` (0.0 -1.0 0.0) :`NewEnumerator3` (0.0 1.0 0.0) :!type "Vector Structure")))

(fn `FocusWidget`
  (params (Widget :type "Widget Object Reference (by ref)"))
  (`WidgetBlueprintLibrary.SetInputMode_GameAndUIEx` (`GameplayStatics.GetPlayerController` null) Widget)
  (return))

(fn `GetGameInstance`
  (returns (GameInstance :type "/Game/Blueprints/Core/GI_Global Object Reference"))
  (bind _asgi_global (cast `/Game/Blueprints/Core/GI_Global` (`GameplayStatics.GetGameInstance` null))
    (:`then`
      (return _asgi_global))
    (:`CastFailed`
      (`self.Print` "NewEnumerator0" "Failed to cast Game Instance" 5.0))))

(fn `Lerp3Color`
  (params (Colors :type "Array of LinearColor Structure") (Alpha :type "Float (double-precision)") (Interval :type "FloatInterval Structure"))
  (returns (`Output Color` :type "LinearColor Structure"))
  (bind (_min _max) (break `FloatInterval` Interval))
  (bind _output (`|GetArrayItem` Colors 1))
  (bind _returnvalue (/ (* (- Alpha _min) 100.0) (* (- _max _min) 100.0)))
  (bind _returnvalue_2 (* _returnvalue 2.0))
  (return (`KismetMathLibrary.SelectColor` (`KismetMathLibrary.LinearColorLerp` (`|GetArrayItem` Colors) _output _returnvalue_2) (`KismetMathLibrary.LinearColorLerp` _output (`|GetArrayItem` Colors 2) _returnvalue_2) (>= _returnvalue 0.5))))

(fn `MouseMoves?`
  (params (OldMousePos :type "Vector2D Structure (by ref)"))
  (returns (`IsMoving?` :type Boolean))
  (locals (Flexibility :type "Float (double-precision)" :default 10.0) (`IsMouseMoving?` :type Boolean))
  (bind (_x _y) (`KismetMathLibrary.BreakVector2D` OldMousePos))
  (bind _returnvalue (`WidgetLayoutLibrary.GetMousePositionOnViewport` null))
  (set `local.IsMouseMoving?` (>= (+ (`KismetMathLibrary.Abs` (- _x (`KismetMathLibrary.BreakVector2D` _returnvalue))) (`KismetMathLibrary.Abs` (- _y (`.Y` (`KismetMathLibrary.BreakVector2D` _returnvalue))))) (`local.Flexibility`)))
  (`KismetMathLibrary.Set2D` (`local.OldMousePos`) (`KismetMathLibrary.BreakVector2D` _returnvalue) (`.Y` (`KismetMathLibrary.BreakVector2D` _returnvalue)))
  (return (`local.IsMouseMoving?`)))

(fn `Pause/Unpause`
  (params (`Pause?` :type Boolean) (WidgetToFocus :type "Widget Object Reference (by ref)") (`ControllerConnected?` :type Boolean))
  (returns (`IsPaused?` :type Boolean))
  (bind _returnvalue (`GameplayStatics.GetPlayerCharacter` null))
  (bind _returnvalue_2 (`GameplayStatics.GetPlayerController` null))
  (if `Pause?`
    (`Actor.DisableInput` _returnvalue _returnvalue_2)
    (`WidgetBlueprintLibrary.SetInputMode_GameAndUIEx` _returnvalue_2 WidgetToFocus)
    (if (not `ControllerConnected?`)
      (set `PlayerController.bShowMouseCursor` true _returnvalue_2))
    (else
      (`Actor.EnableInput` _returnvalue _returnvalue_2)
      (`WidgetBlueprintLibrary.SetInputMode_GameOnly` _returnvalue_2)
      (set `PlayerController.bShowMouseCursor` false _returnvalue_2)))
  (return (`local.Pause?`)))

(fn `Print`
  (params (Type :type "/Game/Blueprints/Enums/E_PrintTypes Enum" :default "NewEnumerator0") (Message :type String :default "Message") (`Duration (in sec)` :type "Float (double-precision)" :default 2.0))
  (`KismetSystemLibrary.PrintString` null (select `bool` (`|EnumInequality` Type "NewEnumerator4") :`false` (`local.Message`) :`true` (`KismetStringLibrary.Concat_StrStr` "[" (`|GetEnumeratorNameAsString` (`local.Type`)) "]" (`local.Message`))) true true (select `/Game/Blueprints/Enums/E_PrintTypes` (`local.Type`) :`NewEnumerator0` (struct :`R` 1.0 :`A` 1.0) :`NewEnumerator1` (struct :`R` 1.0 :`G` 1.0 :`A` 1.0) :`NewEnumerator2` (struct :`G` 1.0 :`B` 1.0 :`A` 1.0) :`NewEnumerator3` (struct :`G` 1.0 :`A` 1.0) :`NewEnumerator4` (struct :`R` 1.0 :`G` 1.0 :`B` 1.0 :`A` 1.0) :!type "LinearColor Structure") (`local.Duration (in sec)`)))

(fn `VectorToEDirection`
  (params (Vector :type "Vector Structure"))
  (returns (Direction :type "/Game/Blueprints/Enums/E_Direction Enum"))
  (return (select `bool` (== Vector_Y 1.0) :`false` (select `bool` (== Vector_X -1.0) :`false` (select `bool` (== Vector_X 1.0) :`false` "NewEnumerator2" :`true` "NewEnumerator0" :!type "/Game/Blueprints/Enums/E_Direction Enum") :`true` "NewEnumerator1") :`true` "NewEnumerator3")))