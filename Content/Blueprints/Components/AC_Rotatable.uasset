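; Actor component that makes its owner rotatable by actors that have AC_CanInteract.
; On BeginPlay it adds a cell-sized box collider and a hidden screen-space WBP_Push widget to the owner at runtime.
; While Active, overlaps from those actors toggle CanBeRotate and the prompt's visibility.
; Rotate checks only Active, then calls RotateMessage on the owner, leaving the rotation itself to that actor.
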(event `self.ReceiveBeginPlay`
  (`self.SetInteractivesAreas`)
  (`self.SetWidget`))

(fn `BeginOverlap`
  (params (OverlappedComponent :type "PrimitiveComponent Object Reference") (OtherActor :type "Actor Object Reference") (OtherComp :type "PrimitiveComponent Object Reference") (OtherBodyIndex :type Integer) (bFromSweep :type Boolean) (SweepResult :type "HitResult Structure (by ref)"))
  (if (`self.Active?`)
    (`/Engine/EditorBlueprintResources/StandardMacros.IsValid` (`Actor.GetComponentByClass` OtherActor "/Game/Blueprints/Components/AC_CanInteract.AC_CanInteract_C")
      (:`Is Valid`
        (set `self.CanBeRotate?` true)
        (`SceneComponent.SetVisibility` (`self.WidgetRef`) true false)
        (return)))))

(fn `EndOverlap`
  (params (OverlappedComponent :type "PrimitiveComponent Object Reference") (OtherActor :type "Actor Object Reference") (OtherComp :type "PrimitiveComponent Object Reference") (OtherBodyIndex :type Integer))
  (if (`self.Active?`)
    (`/Engine/EditorBlueprintResources/StandardMacros.IsValid` (`Actor.GetComponentByClass` OtherActor "/Game/Blueprints/Components/AC_CanInteract.AC_CanInteract_C")
      (:`Is Valid`
        (set `self.CanBeRotate?` false)
        (`SceneComponent.SetVisibility` (`self.WidgetRef`) false false)
        (return)))))

(fn `Rotate`
  (if (`self.Active?`)
    (message `/Game/Blueprints/Interfaces/BPI_Rotation.Rotate` (`self.GetOwner`))))

(fn `SetInteractivesAreas`
  (bind _cellsize (`self.CellSize`))
  ;[1 1 1] Add the 4 Box colliders
  (bind _returnvalue (`|AddComponentByClass` (`self.GetOwner`) "/Script/Engine.BoxComponent" false (`KismetMathLibrary.MakeTransform` (`KismetMathLibrary.MakeVector` 0.0 0.0 (/ _cellsize 2.0)) (struct) (`KismetMathLibrary.Conv_DoubleToVector` (* (/ _cellsize 64.0) 2.0)))))
  ;[1 1 1] Set Options for Box colliders
  (`PrimitiveComponent.SetCollisionResponseToChannel` _returnvalue "ECC_GameTraceChannel5" "ECR_Ignore")
  (`SceneComponent.SetHiddenInGame` _returnvalue (`self.BoxHidden?`) false)
  ;[1 1 1] Bind Events for the Box colliders
  (add `PrimitiveComponent.OnComponentBeginOverlap` _returnvalue (`|CreateDelegate` :!event `BeginOverlap`))
  (add `PrimitiveComponent.OnComponentEndOverlap` _returnvalue (`|CreateDelegate` :!event `EndOverlap`)))

(fn `SetWidget`
  (bind _returnvalue (`|AddComponentByClass` (`self.GetOwner`) "/Script/UMG.WidgetComponent" false (`KismetMathLibrary.MakeTransform` (`KismetMathLibrary.MakeVector` 0.0 0.0 (* (`self.CellSize`) 1.1)))))
  (bind _output_get (set `self.WidgetRef` _returnvalue))
  (`SceneComponent.SetVisibility` _output_get false false)
  (`WidgetComponent.SetWidgetSpace` _output_get "Screen")
  (`PrimitiveComponent.SetCollisionEnabled` _output_get "NoCollision")
  (bind _returnvalue_2 (`|CreateWidget` "/Game/Blueprints/Widgets/WBP_Push.WBP_Push_C" (`GameplayStatics.GetPlayerController` 0)))
  (`WidgetComponent.SetWidget` _output_get _returnvalue_2))