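; AC_CanInteract is an actor component that lets its owner interact with movable and rotatable objects directly in front of it.
; Each of its two events runs a small sphere trace from the owner along its forward vector, out to InteractAreaSize, on a dedicated trace channel.
; InteractForward calls Move on the hit actor's AC_Movable component, while InteractForward2 calls Rotate on its AC_Rotatable, each only if that component exists.
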(event `InteractForward`
  (bind _returnvalue (`self.GetOwner`))
  (bind _returnvalue_2 (`Actor.K2_GetActorLocation` _returnvalue))
  (bind (_outhit _returnvalue_3) (`KismetSystemLibrary.SphereTraceSingle` _returnvalue_2 (+ _returnvalue_2 (* (`Actor.GetActorForwardVector` _returnvalue) (`self.InteractAreaSize`))) 2.0 "TraceTypeQuery6" false (`|MakeArray` _returnvalue)))
  (if _returnvalue_3
    (bind _returnvalue_4 (`Actor.GetComponentByClass` (`.HitActor` (`GameplayStatics.BreakHitResult` _outhit)) "/Game/Blueprints/Components/AC_Movable.AC_Movable_C"))
    (`/Engine/EditorBlueprintResources/StandardMacros.IsValid` _returnvalue_4
      (:`Is Valid`
        (`/Game/Blueprints/Components/AC_Movable.Move` _returnvalue_4)))))

(event `InteractForward2`
  (bind _returnvalue (`self.GetOwner`))
  (bind _returnvalue_2 (`Actor.K2_GetActorLocation` _returnvalue))
  (bind (_outhit _returnvalue_3) (`KismetSystemLibrary.SphereTraceSingle` _returnvalue_2 (+ _returnvalue_2 (* (`Actor.GetActorForwardVector` _returnvalue) (`self.InteractAreaSize`))) 2.0 "TraceTypeQuery6" false (`|MakeArray` _returnvalue)))
  (if _returnvalue_3
    (bind _returnvalue_4 (`Actor.GetComponentByClass` (`.HitActor` (`GameplayStatics.BreakHitResult` _outhit)) "/Game/Blueprints/Components/AC_Rotatable.AC_Rotatable_C"))
    (`/Engine/EditorBlueprintResources/StandardMacros.IsValid` _returnvalue_4
      (:`Is Valid`
        (`/Game/Blueprints/Components/AC_Rotatable.Rotate` _returnvalue_4)))))