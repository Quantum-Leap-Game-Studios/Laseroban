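; Actor component that makes its owner a pushable, grid-based cube the player can move one cell at a time.
; Spawns four side trigger boxes and a screen-space push widget, shown when an AC_CanInteract actor overlaps a side, which also sets the direction.
; Move line-traces one cell opposite that side and, if clear, sends the target to the owner via MoveMessage.
; A looping timer rechecks player overlaps.
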(event `self.ReceiveBeginPlay`
  (`self.SetInteractivesAreas`)
  (`self.SetWidget`))

(event `Move`
  (if (`self.Active?`)
    ;[1 1 1] Check if the player is close to the cube
    (if (`self.CanBeMoved?`)
      (if (not (`self.Moving?`))
        (`self.MoveTo`)
        (else
          (`/Game/Blueprints/Libraries/BLF_Convert.Print` "NewEnumerator1" "[Warning] - Already moving !")))
      (else
        (`/Game/Blueprints/Libraries/BLF_Convert.Print` "NewEnumerator1" "[Warning] - Not enough close !")))))

(fn `BeginOverlap`
  (params (OverlappedComponent :type "PrimitiveComponent Object Reference") (OtherActor :type "Actor Object Reference") (OtherComp :type "PrimitiveComponent Object Reference") (OtherBodyIndex :type Integer) (bFromSweep :type Boolean) (SweepResult :type "HitResult Structure (by ref)"))
  (bind _cellsize (`self.CellSize`))
  (bind _returnvalue (/ _cellsize (/ 4.0 3.0)))
  (if (`self.Active?`)
    (`/Engine/EditorBlueprintResources/StandardMacros.IsValid` (`Actor.GetComponentByClass` OtherActor "/Game/Blueprints/Components/AC_CanInteract.AC_CanInteract_C")
      (:`Is Valid`
        (set `self.CanBeMoved?` true)
        (set `self.CurrentDirection` (`/Game/Blueprints/Libraries/BLF_Convert.VectorToEDirection` (/ (`SceneComponent.RelativeLocation` OverlappedComponent) (`KismetMathLibrary.MakeVector` _returnvalue _returnvalue (/ _cellsize 2.0)))))
        (`SceneComponent.SetVisibility` (`self.WidgetRef`) true false)
        (return)))))

(fn `CheckOverlap`
  (bind _returnvalue (`GameplayStatics.GetPlayerCharacter` 0))
  (for _array_element (`self.BoxesColliders`)
    (if (`PrimitiveComponent.IsOverlappingActor` _array_element _returnvalue)
      (`self.BeginOverlap` _array_element _returnvalue))))

(fn `EndOverlap`
  (params (OverlappedComponent :type "PrimitiveComponent Object Reference") (OtherActor :type "Actor Object Reference") (OtherComp :type "PrimitiveComponent Object Reference") (OtherBodyIndex :type Integer))
  (bind _cellsize (`self.CellSize`))
  (bind _returnvalue (/ _cellsize (/ 4.0 3.0)))
  (if (`self.Active?`)
    (`/Engine/EditorBlueprintResources/StandardMacros.IsValid` (`Actor.GetComponentByClass` OtherActor "/Game/Blueprints/Components/AC_CanInteract.AC_CanInteract_C")
      (:`Is Valid`
        (if (`|EnumEquality` (`self.CurrentDirection`) (`/Game/Blueprints/Libraries/BLF_Convert.VectorToEDirection` (/ (`SceneComponent.RelativeLocation` OverlappedComponent) (`KismetMathLibrary.MakeVector` _returnvalue _returnvalue (/ _cellsize 2.0)))))
          (set `self.CanBeMoved?` false)
          (`SceneComponent.SetVisibility` (`self.WidgetRef`) false false)
          (return))))))

(fn `GetDirection`
  (returns (Direction :type "/Game/Blueprints/Enums/E_Direction Enum"))
  (return (`self.CurrentDirection`)))

(fn `GetMoving?`
  (returns (`Moving?` :type Boolean))
  (return (`self.Moving?`)))

(fn `MoveTo`
  (bind _returnvalue (`self.GetOwner`))
  (bind _returnvalue_2 (`self.GetOwner`))
  (bind _returnvalue_3 (`Actor.K2_GetActorLocation` _returnvalue_2))
  ;[1 1 1] Check if there is nothing in front of the cube
  (bind (_outhit _returnvalue_4) (`KismetSystemLibrary.LineTraceSingle` _returnvalue_3 (+ _returnvalue_3 (* (`/Game/Blueprints/Libraries/BLF_Convert.EDirectionToVector` (`self.CurrentDirection`)) (* (`self.CellSize`) -1.0))) "TraceTypeQuery6" false (`|MakeArray` _returnvalue_2) "None" true (struct :`G` 0.047309 :`B` 1.0 :`A` 1.0) (struct :`R` 1.0 :`B` 0.528396 :`A` 1.0) 20.0))
  (if _returnvalue_4
    ;[1 1 1] Reset if blocked
    (`/Game/Blueprints/Libraries/BLF_Convert.Print` "NewEnumerator1" "[Warning] - Blocked !")
    (set `self.Moving?` false)
    (else
      ;[1 1 1] Move to the next case
      (set `self.Moving?` true)
      (message `/Game/Blueprints/Interfaces/BPI_Movement.Move` _returnvalue (+ (`Actor.K2_GetActorLocation` _returnvalue) (* (`/Game/Blueprints/Libraries/BLF_Convert.EDirectionToVector` (`self.CurrentDirection`)) (* (`self.CellSize`) -1.0)))))))

(fn `SetInteractivesAreas`
  (bind _cellsize (`self.CellSize`))
  (bind _returnvalue (/ _cellsize 64.0))
  (bind _returnvalue_2 (/ _returnvalue 2.0))
  ;[1 1 1] Add the 4 Box colliders
  (bind _enumvalue (foreach `/Game/Blueprints/Enums/E_Direction` false)
    (:`LoopBody`
      (bind _return_value (`/Game/Blueprints/Libraries/BLF_Convert.EDirectionOnXAxis` _enumvalue))
      (bind _returnvalue_3 (`|AddComponentByClass` (`self.GetOwner`) "/Script/Engine.BoxComponent" false (`KismetMathLibrary.MakeTransform` (+ (* (`/Game/Blueprints/Libraries/BLF_Convert.EDirectionToVector` _enumvalue) (/ _cellsize (/ 4.0 3.0))) (`KismetMathLibrary.MakeVector` 0.0 0.0 (/ _cellsize 2.0))) (struct) (`KismetMathLibrary.MakeVector` (`KismetMathLibrary.SelectFloat` _returnvalue_2 _returnvalue _return_value) (`KismetMathLibrary.SelectFloat` _returnvalue _returnvalue_2 _return_value) _returnvalue))))
      ;[1 1 1] Set Options for Box colliders
      (`PrimitiveComponent.SetCollisionResponseToChannel` _returnvalue_3 "ECC_GameTraceChannel5" "ECR_Ignore")
      (`SceneComponent.SetHiddenInGame` _returnvalue_3 (`self.BoxHidden?`) false)
      ;[1 1 1] Bind Events for the Box colliders
      (add `PrimitiveComponent.OnComponentBeginOverlap` _returnvalue_3 (`|CreateDelegate` :!event `BeginOverlap`))
      (add `PrimitiveComponent.OnComponentEndOverlap` _returnvalue_3 (`|CreateDelegate` :!event `EndOverlap`))
      (`KismetArrayLibrary.Array_AddUnique` (`self.BoxesColliders`) _returnvalue_3))
    (:`then`
      ;[1 1 1] Check Overlap boxes colliders
      (`KismetSystemLibrary.K2_SetTimerDelegate` (`|CreateDelegate` :!event `CheckOverlap`) 0.25 true true))))

(fn `SetMoving?`
  (params (`NewMoving?` :type Boolean))
  (set `self.Moving?` `NewMoving?`)
  (return))

(fn `SetWidget`
  (bind _returnvalue (`|AddComponentByClass` (`self.GetOwner`) "/Script/UMG.WidgetComponent" false (`KismetMathLibrary.MakeTransform` (`KismetMathLibrary.MakeVector` 0.0 0.0 (* (`self.CellSize`) 0.9)))))
  (bind _output_get (set `self.WidgetRef` _returnvalue))
  (`SceneComponent.SetVisibility` _output_get false false)
  (`WidgetComponent.SetWidgetSpace` _output_get "Screen")
  (`PrimitiveComponent.SetCollisionEnabled` _output_get "NoCollision")
  (bind _returnvalue_2 (`|CreateWidget` "/Game/Blueprints/Widgets/WBP_Push.WBP_Push_C" (`GameplayStatics.GetPlayerController` 0)))
  (`WidgetComponent.SetWidget` _output_get _returnvalue_2))