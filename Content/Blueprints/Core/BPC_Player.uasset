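; Player controller Blueprint that sets up Enhanced Input mappings and detects whether the player is using gamepad or keyboard and mouse.
; On BeginPlay it clears and re-adds mapping contexts from getters; keyboard returns IMC_Default, while the controller getter returns none.
; Key presses and per-tick mouse movement update ControllerConnected.
; In menus, a mismatch fires the connect/disconnect dispatcher and shows the cursor only without a gamepad.
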(event `UpdateMapping`
  (bind _returnvalue (pcsubsystem `EnhancedInputLocalPlayerSubsystem` self))
  ;[1 1 1] Mapping | Keyboard/Controller
  (`EnhancedInputSubsystemInterface.ClearAllMappings` _returnvalue)
  (`EnhancedInputSubsystemInterface.AddMappingContext` _returnvalue (`self.GetKeyboardMapping`) 0 (struct))
  (`EnhancedInputSubsystemInterface.AddMappingContext` _returnvalue (`self.GetControllerMapping`) 0 (struct)))

(event `Key|AnyKey` :paused true
  (params (Key :type "Key Structure"))
  ;[1 1 1] Mapping | Keyboard/Controller
  ;;[0.588 1 0] Controller Check
  (:`Pressed`
    (`self.HandleKeyPressed` Key)
    (if (== (`self.bShowMouseCursor`) (`self.ControllerConnected?`)) :!label _label
      (if (`self.InMenu?`)
        (`self.Connect/DisconnectController`)
        (set `self.bShowMouseCursor` (not (`self.ControllerConnected?`)))))))

(event `self.ReceiveTick`
  (params (DeltaSeconds :type "Float (single-precision)"))
  ;[1 1 1] Mapping | Keyboard/Controller
  ;;[0.588 1 0] Controller Check
  (`self.HandleMouseMoved`)
  (goto _label))

(event `self.ReceiveBeginPlay`
  (`self.UpdateMapping`))

(fn `GetControllerMapping`
  (returns (MappingContext :type "InputMappingContext Object Reference"))
  (return null))

(fn `GetKeyboardMapping`
  (returns (MappingContext :type "InputMappingContext Object Reference"))
  (return "/Game/Inputs/IMC_Default.IMC_Default"))

(fn `UserConstructionScript`)