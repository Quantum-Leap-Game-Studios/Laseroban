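; HUD_Player is the player HUD Blueprint that owns and toggles the pause menu.
; On BeginPlay it creates a WBP_Pause widget for the first player controller, adds it to the viewport collapsed and binds its resume-click event.
; PauseUnpause shows the widget and focuses its first element, or collapses it, without changing game pause state itself.
; Clicking resume calls PauseUnpause to hide the menu.
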(event `self.ReceiveBeginPlay`
  (bind _returnvalue (`|CreateWidget` "/Game/Blueprints/Widgets/Menu/WBP_Pause.WBP_Pause_C" (`GameplayStatics.GetPlayerController` 0)))
  (bind _output_get (set `self.PauseRef` _returnvalue))
  (`UserWidget.AddToViewport` _output_get 0)
  (`Widget.SetVisibility` _output_get "Collapsed")
  (add `/Game/Blueprints/Widgets/Menu/WBP_Pause.OnResumeClicked` _output_get (delegate `OnResumeClicked`)))

(event `OnResumeClicked`
  (bind _ispaused_ (`/Game/Blueprints/Libraries/BLF_Convert.Pause/Unpause` false))
  (`self.Pause/Unpause` _ispaused_))

(fn `Pause/Unpause`
  (params (`Pause?` :type Boolean))
  (bind _pauseref (`self.PauseRef`))
  (if `Pause?`
    (`Widget.SetVisibility` _pauseref "Visible")
    (`/Game/Blueprints/Widgets/Menu/WBP_Pause.FocusOnFirstElem` _pauseref)
    (else
      (`Widget.SetVisibility` _pauseref "Collapsed")))
  (return))

(fn `UserConstructionScript`)