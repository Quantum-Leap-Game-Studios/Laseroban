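; AC_Hold is an actor component that lets the player pick up and drop physics objects with the interact input.
; On BeginPlay it adds the interaction mapping context and caches the owner's physics constraint, using that constraint's parent static mesh as the anchor slot.
; Interacting box-traces from the camera and constrains any hit simulating component (with bone name) to the anchor, or breaks the constraint if something is already held.
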(event `self.ReceiveBeginPlay`
  ;[1 1 1] Start by adding the inputs for this component
  (`EnhancedInputSubsystemInterface.AddMappingContext` (pcsubsystem `EnhancedInputLocalPlayerSubsystem` (`GameplayStatics.GetPlayerController` 0)) "/Game/Lasers/HoldObject/IMC_Interaction.IMC_Interaction" 0 (struct))
  (bind _output_get (set `self.Physics Constraint` (`Actor.GetComponentByClass` (`self.GetOwner`) "/Script/Engine.PhysicsConstraintComponent"))) ; Save physics constraint component
  ;[1 1 1] Get the parent component of the physics constraint (it is necessary to act as an anchor)
  (bind _asstatic_mesh_component (cast `StaticMeshComponent` (`|GetArrayItem` (`SceneComponent.GetParentComponents` _output_get))))
  (set `self.HeldObjectSlot` _asstatic_mesh_component))

(event `EnhancedInput|/Game/Lasers/HoldObject/IA_Interact`
  (params (ActionValue :type Boolean) (ElapsedSeconds :type "Float (double-precision)") (TriggeredSeconds :type "Float (double-precision)") (InputAction :type "InputAction Object Reference" :default "/Game/Lasers/HoldObject/IA_Interact.IA_Interact"))
  (bind _returnvalue (`GameplayStatics.GetPlayerCameraManager` 0))
  ;[1 1 1] Player presses input to pick up objects
  (:`Triggered`
    (`self.Trace For Pickup` (`Actor.K2_GetActorLocation` _returnvalue) (`Actor.GetActorForwardVector` _returnvalue) 300.0)))

(fn `Pickup Object`
  (params (`P-HitResult` :type "HitResult Structure"))
  (bind (_bblockinghit _binitialoverlap _time _distance _location _impactpoint _normal _impactnormal _physmat _hitactor _hitcomponent _hitbonename _bonename) (`GameplayStatics.BreakHitResult` `P-HitResult`))
  ;[1 1 1] Only perform the rest if the actor hit is simulating physics
  (if (`SceneComponent.IsSimulatingPhysics` _hitcomponent "None")
    ;[1 1 1] This forces the hit component to be linked to the physics constraint component (if the component 1 is a character you can set a bone name as well)
    (`PhysicsConstraintComponent.SetConstrainedComponents` (`self.Physics Constraint`) (`self.HeldObjectSlot`) "None" _hitcomponent _bonename)
    (set `self.Held Object` _hitcomponent) ; Assign the newly picked up object\nto the Held Object for the TraceForPickup\nto know that an object is held
  ))

(fn `Release Object`
  (`PhysicsConstraintComponent.BreakConstraint` (`self.Physics Constraint`)) ; Releases the object from the players "hands"
  (set `self.Held Object` null) ; Cleared so that the trace for pickup knows\nthat the actor has been dropped
)

(fn `Trace For Pickup`
  (params (`P-StartLocation` :type "Vector Structure") (`P-ForwardVector` :type "Vector Structure") (`P-Range` :type "Float (double-precision)"))
  (bind _p_startlocation (`local.P-StartLocation`))
  (`self.Held Object` ; Is this component currently holding an object\nor not?
    (:`then`
      (`self.Release Object`))
    (:`else`
      ;[1 1 1] Box trace in front of player camera and pickup object if something was hit
      (bind (_outhit _returnvalue) (`KismetSystemLibrary.BoxTraceSingle` _p_startlocation (+ _p_startlocation (* (`local.P-ForwardVector`) (`local.P-Range`))) (20.0 20.0 20.0) (struct) "TraceTypeQuery1"))
      (if _returnvalue
        (`self.Pickup Object` _outhit)))))